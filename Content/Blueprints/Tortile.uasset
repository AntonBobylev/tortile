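; Tortile is a moving entity that travels in a straight line from where it is placed to a destination point, then destroys itself.
; BeginPlay plays an attached walking sound and a brief spawn effect, while construction sets the spawn and destroy sounds used alongside parent logic.
; Tick moves it at constant speed, spawning a walk emitter every frame.
; On arrival it notifies its SpawningSpot, shows a destroy effect and calls DestroyEntity after a short delay.
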(event `self.ReceiveBeginPlay`
  (`parent.ReceiveBeginPlay`)
  (`GameplayStatics.SpawnSoundAttached` "/Game/Sounds/tortile_walk_sound.tortile_walk_sound" (`self.WalkingSound`) "None" (0.0 0.0 0.0) (struct) "KeepRelativeOffset" true 1.0 1.0 0.0 null null)
  (bind _returnvalue (`GameplayStatics.SpawnEmitterAtLocation` (`self.tortileSpawnEffect`) (`SceneComponent.K2_GetComponentLocation` (`self.Tortile`)) (struct) (0.2 0.2 0.2)))
  (`KismetSystemLibrary.Delay` 0.5)
  (`ActorComponent.Deactivate` _returnvalue))

(event `self.ReceiveTick`
  (params (DeltaSeconds :type "Float (single-precision)"))
  (`parent.ReceiveTick` DeltaSeconds)
  (if (and (`self.canMove`) (not (`self.isInDestinationPoint`)))
    (`self.Move` DeltaSeconds)
    (`GameplayStatics.SpawnEmitterAttached` (`self.tortileWalkEffect`) (`self.Tortile`) "None" (0.0 0.0 0.0) (struct) (0.1 0.2 0.1))
    (bind _yes (`self.NeedToDestroy`))
    (if _yes
      (`/Game/Blueprints/TortileSpawningSpot.TortileIsInDestinationPoint` (`self.spawningSpot`))
      (set `self.isInDestinationPoint` true)
      (`self.SpawnDestroyEffect`)
      (`KismetSystemLibrary.Delay` 0.5)
      (`self.Destroy Entity`))))

(fn `Move`
  (params (DeltaSeconds :type "Float (double-precision)"))
  (locals (FrameTime :type "Float (double-precision)"))
  (set `local.FrameTime` DeltaSeconds)
  (bind _output_get (set `self.currentPosition` (`KismetMathLibrary.VInterpTo_Constant` (`self.currentPosition`) (`self.destinationPoint`) (`local.FrameTime`) (`self.speed`))))
  (`self.K2_SetActorLocation` _output_get)
  (set `self.isMoving` true))

(fn `NeedToDestroy`
  (returns (Yes :type Boolean))
  (return (== (`self.currentPosition`) (`self.destinationPoint`))))

(fn `SpawnDestroyEffect`
  (`GameplayStatics.SpawnEmitterAttached` (`self.tortileDestroyEffect`) (`self.Tortile`) "None" (0.0 0.0 0.0) (struct) (0.1 0.1 0.1)))

(fn `UserConstructionScript`
  (set `self.spawnSound` "/Game/Sounds/tortile_spawn_sound.tortile_spawn_sound")
  (`parent.UserConstructionScript`)
  (set `self.canMove` true)
  (set `self.currentPosition` (`self.K2_GetActorLocation`))
  (set `self.destroySound` "/Game/Sounds/tortile_destroy_sound.tortile_destroy_sound")
  (set `self.walkSound` null))