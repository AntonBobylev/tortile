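; SpawningSpot is an actor that spawns Tortile actors and sends them toward a linked destination spot.
; Its Spawn event checks CanSpawnEntities, set true at construction, then spawns the configured class at the SpawnPoint component's location.
; Each spawned Tortile receives the DestinationSpot's DestPoint location and a reference back to this spot.
; The TortileIsinDestinationPoint event tells the linked Button that it can spawn again.
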(event `self.Spawn`
  (if (`self.canSpawnEntities`)
    (`self.SpawnTortile`)))

(event `/Game/Blueprints/TortileSpawningSpot.TortileIsInDestinationPoint`
  (`self.CanSpawnAgain` (`self.Button`)))

(fn `SpawnTortile`
  (bind _returnvalue (`|SpawnActorFromClass` (`self.TortileToSpawn`) (`KismetMathLibrary.MakeTransform` (`SceneComponent.K2_GetComponentLocation` (`self.spawnPoint`))) "Undefined" "OverrideRootScale" null null))
  (set `/Game/Blueprints/Tortile.destinationPoint` (`SceneComponent.K2_GetComponentLocation` (`/Game/Blueprints/DestSpot.DestPoint` (`self.DestinationSpot`))) _returnvalue)
  (set `/Game/Blueprints/Tortile.spawningSpot` self _returnvalue))

(fn `UserConstructionScript`
  (`parent.UserConstructionScript`)
  (set `self.canSpawnEntities` true))