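; SecondSpotTortile is an actor Blueprint with movement logic that alternates between travelling toward a destination and pausing.
; Move accumulates a go timer and calls DoMove, which steps the location at constant speed via VInterpToConstant without sweeping.
; Once the go time expires, DoStop runs a stop timer that resets both timers after the pause.
; Tick only calls its parent, and nothing in this graph calls Move.
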(event `self.ReceiveTick`
  (params (DeltaSeconds :type "Float (single-precision)"))
  (`parent.ReceiveTick` DeltaSeconds))

(fn `DoMove`
  (params (DestinationPoint :type "Vector Structure"))
  (bind _output_get (set `self.currentPosition` (`KismetMathLibrary.VInterpTo_Constant` (`self.currentPosition`) DestinationPoint (`self.Frame Time`) (`self.speed`))))
  (`self.K2_SetActorLocation` _output_get))

(fn `DoStop`
  (`self.IncreaseStopTimer`)
  (`self.ResetTimers`)
  (set `self.isMoving` false))

(fn `IncreaseGoTimer`
  (set `self.GoTimer` (+ (`self.Frame Time`) (`self.GoTimer`))))

(fn `IncreaseStopTimer`
  (set `self.StopTimer` (+ (`self.StopTimer`) (`self.Frame Time`))))

(fn `Move`
  (params (DeltaSeconds :type "Float (double-precision)"))
  (set `self.Frame Time` DeltaSeconds)
  (`self.IncreaseGoTimer`)
  (bind _yes (`self.TimeIsOver`))
  (bind _output_get (set `self.isMoving` _yes))
  (if _output_get
    (`self.DoStop`)
    (else
      (`self.DoMove` (`self.destinationPoint`)))))

(fn `ResetTimers`
  (if (>= (`self.StopTimer`) (`self.TimeToGo`))
    (set `self.StopTimer` 0.0)
    (set `self.GoTimer` 0.0)))

(fn `TimeIsOver`
  (returns (Yes :type Boolean))
  (return (>= (`self.GoTimer`) (`self.TimeToStop`))))

(fn `UserConstructionScript`
  (`parent.UserConstructionScript`))