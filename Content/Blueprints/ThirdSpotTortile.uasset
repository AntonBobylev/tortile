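; ThirdSpotTortile is an actor Blueprint that moves toward a destination point for a timed period, then heads back to its spawning spot.
; Move stores the frame time, advances a go timer and calls DoMove toward the destination until TimeIsOver returns true.
; DoRevertMove then moves it toward the spawning spot's location, advances a stop timer and calls ResetTimers.
; The event graph holds only disabled default events, so nothing in this file calls Move.
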(fn `DoRevertMove`
  (`self.DoMove` (`self.K2_GetActorLocation` (`self.spawningSpot`)))
  (`self.IncreaseStopTimer`)
  (`self.ResetTimers`))

(fn `Move`
  (params (DeltaSeconds :type "Float (double-precision)"))
  (set `self.Frame Time` DeltaSeconds)
  (`self.IncreaseGoTimer`)
  (bind _yes (`self.TimeIsOver`))
  (if _yes
    (`self.DoRevertMove`)
    (else
      (`self.DoMove` (`self.destinationPoint`)))))

(fn `UserConstructionScript`
  (`parent.UserConstructionScript`))