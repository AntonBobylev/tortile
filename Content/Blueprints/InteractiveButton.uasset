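; InteractiveButton is a world button that triggers a spawn when the player stands in its overlap and holds the interaction key.
; Overlap events set PlayerIsNear for the FirstPersonCharacter, and Tick polls the key each frame.
; On press it sends SpawnMessage through the ButtonSpawningSpot interface to its assigned SpawningSpot.
; An EntitySpawned flag blocks repeat spawns until CanSpawnAgain clears it.
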(event `self.ReceiveTick`
  (params (DeltaSeconds :type "Float (single-precision)"))
  (`parent.ReceiveTick` DeltaSeconds)
  (bind _available (`self.spawnIsAvailable`))
  (if _available
    (`self.spawnEntity`)
    (set `self.entitySpawned` true)))

(event `self.ReceiveActorBeginOverlap`
  (params (OtherActor :type "Actor Object Reference"))
  (`self.setPlayerNear` OtherActor true))

(event `self.ReceiveActorEndOverlap`
  (params (OtherActor :type "Actor Object Reference"))
  (`self.setPlayerNear` OtherActor))

(event `/Game/Blueprints/ButtonSpawningSpot.CanSpawnAgain`
  (set `self.entitySpawned` false))

(fn `setPlayerNear`
  (params (PlayerBP :type "Object Object Reference") (BeginOverlap :type Boolean))
  (if (`self.isInteractive`)
    (cast `/Game/FirstPersonBP/Blueprints/FirstPersonCharacter` PlayerBP)
    (set `self.playerIsNear` BeginOverlap)))

(fn `spawnEntity`
  (bind _outactors (`GameplayStatics.GetAllActorsWithInterface` "/Game/Blueprints/ButtonSpawningSpot.ButtonSpawningSpot_C"))
  (for _array_element _outactors
    (if (== _array_element (`self.SpawningSpot`))
      (message `/Game/Blueprints/ButtonSpawningSpot.Spawn` _array_element))))

(fn `spawnIsAvailable`
  (returns (available :type Boolean))
  (return (and (`PlayerController.IsInputKeyDown` (`GameplayStatics.GetPlayerController` 0) (`self.interactionKey`)) (`self.playerIsNear`) (not (`self.entitySpawned`)))))

(fn `UserConstructionScript`
  (`parent.UserConstructionScript`)
  (set `self.isInteractive` true))